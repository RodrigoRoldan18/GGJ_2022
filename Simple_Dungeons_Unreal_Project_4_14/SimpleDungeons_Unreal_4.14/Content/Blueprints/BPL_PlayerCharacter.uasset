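; BPL_PlayerCharacter is an interface-style set of function stubs for the player character, with no logic beyond returning false or zero.
; It covers attack, interaction with a mana consumption value, and a player identity check.
; Other functions read and add health and mana, get and set attacking and repairing states, and toggle repair ability.
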(fn `AddHealth`
  (params (HealthValue :type "Float (double-precision)"))
  (returns (Return :type Boolean))
  (return false))

(fn `AddMana`
  (params (ManaValue :type "Float (double-precision)"))
  (returns (Return :type Boolean))
  (return false))

(fn `Attack`
  (returns (Return :type Boolean))
  (return false))

(fn `EnableRepair`
  (params (CanRepair :type Boolean))
  (returns (Return :type Boolean))
  (return false))

(fn `GetHealth`
  (returns (Health :type "Float (double-precision)"))
  (return 0.0))

(fn `GetIsAttacking`
  (returns (Return :type Boolean))
  (return false))

(fn `GetIsRepairing`
  (returns (Return :type Boolean))
  (return false))

(fn `GetMana`
  (returns (CurrentMana :type "Float (double-precision)"))
  (return 0.0))

(fn `Interact`
  (params (ManaConsumptionValue :type "Float (double-precision)"))
  (returns (Return :type Boolean))
  (return false))

(fn `IsPlayer`
  (returns (IsPlayer :type Boolean))
  (return false))

(fn `SetIsAttacking`
  (params (IsAttacking :type Boolean))
  (returns (Return :type Boolean))
  (return false))

(fn `SetIsRepairing`
  (params (IsRepairing :type Boolean))
  (returns (Return :type Boolean))
  (return false))