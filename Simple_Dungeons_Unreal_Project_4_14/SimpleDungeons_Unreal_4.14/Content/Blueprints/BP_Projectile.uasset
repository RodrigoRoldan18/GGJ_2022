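; Projectile actor, fired by the player or an enemy, that damages opposing characters, with enemy shots also damaging the Objective.
; The construction script checks whether the instigator is the player, switching non-player shots to the enemy role and fireball particles.
; On collision overlap it compares the other actor's role with its own, then applies damage and destroys itself on a valid hit.
; A fireball sound plays in 2D on spawn.
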(event `self.ReceiveBeginPlay`
  (`GameplayStatics.PlaySound2D` "/Game/Sound/Fireball_Cue.Fireball_Cue" 1.0 1.0 0.0 null null))

(event `self.Collision.OnComponentBeginOverlap`
  (params (OverlappedComponent :type "PrimitiveComponent Object Reference") (OtherActor :type "Actor Object Reference") (OtherComp :type "PrimitiveComponent Object Reference") (OtherBodyIndex :type Integer) (bFromSweep :type Boolean) (SweepResult :type "HitResult Structure (by ref)"))
  (bind _actorrole (message `/Game/Blueprints/BPL_Actors.GetActorRole` OtherActor))
  (if (or (`|EnumEquality` _actorrole "NewEnumerator0") (`|EnumEquality` _actorrole "NewEnumerator1"))
    (if (`|EnumInequality` _actorrole (`self.ActorRole`))
      (`GameplayStatics.ApplyDamage` OtherActor (`self.DamageValue`) :!label _label)
      (`self.K2_DestroyActor`))
    (elif (`|EnumEquality` _actorrole "NewEnumerator2")
      (if (`|EnumEquality` (`self.ActorRole`) "NewEnumerator1")
        (goto _label)))))

(fn `UserConstructionScript`
  (bind _isplayer (message `/Game/Blueprints/BPL_PlayerCharacter.IsPlayer` (`self.GetInstigator`)))
  (if (not _isplayer)
    (`ParticleSystemComponent.SetTemplate` (`self.ParticleSystem`) "/Game/VFX/Fireball_PS.Fireball_PS")
    (set `self.ActorRole` "NewEnumerator1")))