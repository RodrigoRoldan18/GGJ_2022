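; Enemy character that takes damage, shows a health bar and, on death, drops a mana orb and prompts the game mode to try starting a new wave.
; A widget health bar starts hidden, appears on damage and stays visible, with Tick updating its fill from Health.
; Role and attack-state functions use real variables, while player-oriented functions for mana, repair, interaction and Attack are stubs, apparently from a shared interface.
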(event `self.ReceiveBeginPlay`
  (`SceneComponent.SetVisibility` (`self.HealthBar`) false false))

(event `self.ReceiveTick`
  (params (DeltaSeconds :type "Float (single-precision)"))
  (bind _asenemy_health (cast `/Game/UI/Widgets/EnemyHealth` (`WidgetComponent.GetWidget` (`self.HealthBar`))))
  (`ProgressBar.SetPercent` (`/Game/UI/Widgets/EnemyHealth.ProgressBar_0` _asenemy_health) (/ (`self.Health`) 100.0)))

(event `self.ReceiveAnyDamage`
  (params (Damage :type "Float (single-precision)") (DamageType :type "DamageType Object Reference") (InstigatedBy :type "Controller Object Reference") (DamageCauser :type "Actor Object Reference"))
  (`SceneComponent.SetVisibility` (`self.HealthBar`) true false)
  (bind _output_get (set `self.Health` (- (`self.Health`) Damage)))
  (if (<= _output_get 0.0)
    (`self.Die`)
    (else
      (`KismetSystemLibrary.Delay` 1.0)
      (`SceneComponent.SetVisibility` (`self.HealthBar`) true false))))

(event `CustomEvent`
  (params (Damage :type "Float (double-precision)") (DamageType :type "DamageType Object Reference") (InstigatedBy :type "Controller Object Reference") (DamageCauser :type "Actor Object Reference")))

(fn `AddMana`
  (params (ManaValue :type "Float (double-precision)"))
  (returns (Return :type Boolean))
  (return false))

(fn `Attack`
  (returns (Return :type Boolean))
  (return false))

(fn `Die`
  (`|SpawnActorFromClass` "/Game/Blueprints/BP_ManaOrb.BP_ManaOrb_C" (`self.GetTransform`) "Undefined" "OverrideRootScale" null null)
  (message `/Game/Blueprints/BPL_MainGameMode.TryStartNewWave` (`GameplayStatics.GetGameMode`))
  (`self.K2_DestroyActor`))

(fn `EnableRepair`
  (params (CanRepair :type Boolean))
  (returns (Return :type Boolean))
  (return false))

(fn `GetActorRole`
  (returns (ActorRole :type "/Game/Blueprints/E_ActorRole Enum"))
  (return (`self.ActorRole`)))

(fn `GetIsAttacking`
  (returns (Return :type Boolean))
  (return (`self.IsAttacking`)))

(fn `GetIsRepairing`
  (returns (Return :type Boolean))
  (return false))

(fn `GetMana`
  (returns (CurrentMana :type "Float (double-precision)"))
  (return 0.0))

(fn `Interact`
  (params (ManaConsumptionValue :type "Float (double-precision)"))
  (returns (Return :type Boolean))
  (return false))

(fn `IsPlayer`
  (returns (IsPlayer :type Boolean))
  (return false))

(fn `SetIsAttacking`
  (params (IsAttacking :type Boolean))
  (returns (Return :type Boolean))
  (set `self.IsAttacking` IsAttacking)
  (return false))

(fn `SetIsRepairing`
  (params (IsRepairing :type Boolean))
  (returns (Return :type Boolean))
  (return false))

(fn `UserConstructionScript`)