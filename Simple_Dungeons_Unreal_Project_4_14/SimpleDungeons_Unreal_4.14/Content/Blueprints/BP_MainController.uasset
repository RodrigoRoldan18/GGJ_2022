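; BP_MainController is a controller that relays player input to whichever pawn it controls.
; Movement axes drive the pawn along the view target's forward and right vectors.
; The Attack action sends AttackMessage to the pawn.
; Tick polls Left Shift directly to open and close a gate, sending InteractMessage with delta seconds each subsequent frame while the key stays held.
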(event `InputAxis|MoveForward`
  (params (AxisValue :type "Float (single-precision)"))
  (`Pawn.AddMovementInput` (`self.K2_GetPawn`) (`self.GetActorForwardVector` (`self.GetViewTarget`)) AxisValue false))

(event `InputAxis|MoveRight`
  (params (AxisValue :type "Float (single-precision)"))
  (`Pawn.AddMovementInput` (`self.K2_GetPawn`) (`self.GetActorRightVector` (`self.GetViewTarget`)) AxisValue false))

(event `InputAction|Attack`
  (params (Key :type "Key Structure"))
  (:`Pressed`
    (message `/Game/Blueprints/BPL_PlayerCharacter.Attack` (`self.K2_GetPawn`))))

(event `self.ReceiveTick`
  (params (DeltaSeconds :type "Float (single-precision)"))
  (if (`self.WasInputKeyJustPressed` "LeftShift")
    (goto _label :!via `Open`)
    (elif (`self.WasInputKeyJustReleased` "LeftShift")
      (goto _label :!via `Close`)
      (else
        (`/Engine/EditorBlueprintResources/StandardMacros.Gate` true :!label _label
          (:`Exit`
            (message `/Game/Blueprints/BPL_PlayerCharacter.Interact` (`self.K2_GetPawn`) DeltaSeconds)))))))

(fn `UserConstructionScript`)