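; Player character Blueprint that fires projectiles and holds a mana pool.
; Attack spawns a BP_Projectile just ahead of the actor along its facing, with itself as instigator, and plays an attack animation directly on the mesh.
; AddMana adds the given value to Mana without clamping.
; IsPlayer identifies the actor as the player, and Interact is an empty stub returning false.
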(fn `AddMana`
  (params (ManaValue :type "Float (double-precision)"))
  (returns (Return :type Boolean))
  (set `self.Mana` (+ ManaValue (`self.Mana`)))
  (return false))

(fn `Attack`
  (returns (Return :type Boolean))
  (`|SpawnActorFromClass` "/Game/Blueprints/BP_Projectile.BP_Projectile_C" (`KismetMathLibrary.MakeTransform` (+ (`self.K2_GetActorLocation`) (* (`self.GetActorForwardVector`) 100.0)) (`self.K2_GetActorRotation`)) "Undefined" "OverrideRootScale" null self)
  (`SkeletalMeshComponent.PlayAnimation` (`self.Mesh`) "/Game/BattleWizardPolyart/Animations/Attack01Anim.Attack01Anim" false)
  (return false))

(fn `Interact`
  (returns (Return :type Boolean))
  (return false))

(fn `IsPlayer`
  (returns (IsPlayer :type Boolean))
  (return true))

(fn `UserConstructionScript`)