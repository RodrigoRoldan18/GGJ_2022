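; Game mode for a wave-based combat game that starts enemy waves and provides aim assist.
; On BeginPlay it caches the objective and all enemy spawners, then spawns the first wave.
; TryStartNewWave triggers every spawner and increments the wave count when at most one enemy remains.
; Aim assist branches on actor role, targeting the nearest enemy or the player (with a wider cone), returning a look-at rotation if within the angle.
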(event `self.ReceiveBeginPlay`
  (`self.InitialiseVariables`)
  (for _array_element (`self.EnemySpawners`)
    (`/Game/Blueprints/BP_EnemySpawner.SpawnNewWave` _array_element)))

(fn `GetCurrentWave`
  (returns (CurrentWave :type Integer))
  (return (`self.CurrentWave`)))

(fn `GetObjective`
  (returns (Objective :type "/Game/Blueprints/BP_Objective Object Reference"))
  (return (`self.Objective`)))

(fn `InitialiseVariables`
  (`|ExecutionSequence`
    (:`then_0`
      (`self.Objective`
        (:`then`)
        (:`else`
          (bind _returnvalue (`GameplayStatics.GetActorOfClass` "/Game/Blueprints/BP_Objective.BP_Objective_C"))
          (set `self.Objective` _returnvalue))))
    (:`then_1`
      (bind _outactors (`GameplayStatics.GetAllActorsOfClass` "/Game/Blueprints/BP_EnemySpawner.BP_EnemySpawner_C"))
      (set `self.EnemySpawners` _outactors))))

(fn `IsWithinAimAssistRange`
  (params (pawnInstigator :type "Pawn Object Reference"))
  (returns (isInRange :type Boolean) (AimAssistRotation :type "Rotator Structure"))
  (locals (Distance :type "Array of Float (double-precision)") (ActiveEnemies :type "Array of /Game/Blueprints/BP_EnemyCharacter Object Reference") (TargetEnemy :type "/Game/Blueprints/BP_EnemyCharacter Object Reference") (VectorBetweenPlayers :type "Vector Structure") (TargetPlayer :type "/Game/Blueprints/BP_PlayerCharacter Object Reference"))
  (bind _pawninstigator (`local.pawnInstigator`))
  (bind _pawninstigator_2 (`local.pawnInstigator`))
  (bind _returnvalue (`self.GetActorForwardVector` _pawninstigator_2))
  (bind _returnvalue_2 (`self.GetActorForwardVector` _pawninstigator))
  (bind _actorrole (message `/Game/Blueprints/BPL_Actors.GetActorRole` pawnInstigator))
  (if (`|EnumEquality` _actorrole "NewEnumerator0")
    (bind _outactors (`GameplayStatics.GetAllActorsOfClass` "/Game/Blueprints/BP_EnemyCharacter.BP_EnemyCharacter_C"))
    (bind _output_get (set `local.ActiveEnemies` _outactors))
    (for _array_element _output_get
      (`KismetArrayLibrary.Array_Add` (`local.Distance`) (`self.GetDistanceTo` _array_element (`local.pawnInstigator`))))
    (bind _output_get_2 (set `local.TargetEnemy` (`|GetArrayItem` (`local.ActiveEnemies`) (`KismetMathLibrary.MinOfFloatArray` (`local.Distance`)))))
    (`local.TargetEnemy`
      (:`then`
        (bind _output_get_3 (set `local.VectorBetweenPlayers` (- (`self.K2_GetActorLocation` _output_get_2) (`self.K2_GetActorLocation` _pawninstigator_2))))
        (if (< (`KismetMathLibrary.DegAcos` (/ (`KismetMathLibrary.Dot_VectorVector` _output_get_3 _returnvalue) (* (`KismetMathLibrary.VSize` (`local.VectorBetweenPlayers`)) (`KismetMathLibrary.VSize` _returnvalue)))) (`self.AimRange`))
          (return true (`KismetMathLibrary.FindLookAtRotation` (`self.K2_GetActorLocation` (`local.pawnInstigator`)) (`self.K2_GetActorLocation` (`local.TargetEnemy`))))
          (else
            (return false))))
      (:`else`))
    (elif (`|EnumEquality` _actorrole "NewEnumerator1")
      (bind _returnvalue_3 (`GameplayStatics.GetActorOfClass` "/Game/Blueprints/BP_PlayerCharacter.BP_PlayerCharacter_C"))
      (bind _output_get_4 (set `local.TargetPlayer` _returnvalue_3))
      (bind _output_get_5 (set `local.VectorBetweenPlayers` (- (`self.K2_GetActorLocation` _output_get_4) (`self.K2_GetActorLocation` _pawninstigator))))
      (if (< (`KismetMathLibrary.DegAcos` (/ (`KismetMathLibrary.Dot_VectorVector` _output_get_5 _returnvalue_2) (* (`KismetMathLibrary.VSize` (`local.VectorBetweenPlayers`)) (`KismetMathLibrary.VSize` _returnvalue_2)))) (* (`self.AimRange`) 1.7))
        (return true (`KismetMathLibrary.FindLookAtRotation` (`self.K2_GetActorLocation` (`local.pawnInstigator`)) (`self.K2_GetActorLocation` (`local.TargetPlayer`))))
        (else
          (return false))))))

(fn `TryStartNewWave`
  (returns (Return :type Boolean))
  (bind _outactors (`GameplayStatics.GetAllActorsOfClass` "/Game/Blueprints/BP_EnemyCharacter.BP_EnemyCharacter_C"))
  (if (<= (`KismetArrayLibrary.Array_Length` _outactors) 1)
    (for _array_element (`self.EnemySpawners`)
      (`/Game/Blueprints/BP_EnemySpawner.SpawnNewWave` _array_element))
    (`/Engine/EditorBlueprintResources/StandardMacros.IncrementInt` (`self.CurrentWave`)
      (:`  `
        (return false)))))

(fn `UserConstructionScript`)